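; Synth manager actor that opens the wavetable synth UI and drives the synth's audio component.
; BeginPlay creates W_Wavetable in UI-only input with a cursor, then loads the "OnConstruct" preset.
; PresetManagement copies a DT_SynthPresets row into the widget controls and SSynthSettings, scaling normalized filter cutoffs into frequencies.
; Tick pushes SSynthSettings to the Audio component's named waveform, filter and ADSR float parameters every frame.
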(event `self.ReceiveBeginPlay`
  (bind _returnvalue (`GameplayStatics.GetPlayerController` 0))
  (bind _returnvalue_2 (`|CreateWidget` "/Game/W_Wavetable.W_Wavetable_C"))
  (bind _output_get (set `self.Wavetable Widget` _returnvalue_2))
  (`UserWidget.AddToViewport` _output_get 0)
  (`WidgetBlueprintLibrary.SetInputMode_UIOnlyEx` _returnvalue _output_get)
  (set `PlayerController.bShowMouseCursor` true _returnvalue)
  (`self.Preset Management` "OnConstruct"))

(event `self.ReceiveTick`
  (params (DeltaSeconds :type "Float (single-precision)"))
  (bind (_s_synth_settings_waveform _s_synth_settings_lowpassfiltercutoff _s_synth_settings_lowpassfilterresonance _s_synth_settings_highpassfiltercutoff _s_synth_settings_highpassfilterresonance _s_synth_settings_waveform2 _s_synth_settings_attack _s_synth_settings_decay _s_synth_settings_sustain _s_synth_settings_release) (break `/Game/S_SynthSettings` (`self.S Synth Settings`)))
  (`self.Synth Settings` _s_synth_settings_waveform _s_synth_settings_lowpassfiltercutoff _s_synth_settings_lowpassfilterresonance _s_synth_settings_highpassfiltercutoff _s_synth_settings_highpassfilterresonance _s_synth_settings_waveform2 _s_synth_settings_attack _s_synth_settings_decay _s_synth_settings_sustain _s_synth_settings_release))

(fn `Preset Management`
  (params (`Preset Row Name` :type Name))
  (bind _wavetable_widget (`self.Wavetable Widget`))
  (bind _returnvalue (`|GetDataTableRow` "/Game/DT_SynthPresets.DT_SynthPresets" `Preset Row Name`)
    (:`then`
      (`Slider.SetValue` (`/Game/W_Wavetable.WaveformSlider` _wavetable_widget) (break `/Game/S_SynthSettings` _returnvalue))
      (`RadialSlider.SetValue` (`/Game/W_Wavetable.LowPassCutOffKnob` _wavetable_widget) (`.LowPassFilterCutOff_4_6D70E24441703CD421BCE9AD6D1FC51C` (break `/Game/S_SynthSettings` _returnvalue)))
      (`RadialSlider.SetValue` (`/Game/W_Wavetable.LowPassResKnob` _wavetable_widget) (`.LowPassFilterResonance_6_EA6623A744C3E250F1A0209D804692E1` (break `/Game/S_SynthSettings` _returnvalue)))
      (`RadialSlider.SetValue` (`/Game/W_Wavetable.HighPassCutOffKnob` _wavetable_widget) (`.HighPassFilterCutOff_9_4D30AA4845A6E9CCB262F3A5AFD4EBD4` (break `/Game/S_SynthSettings` _returnvalue)))
      (`RadialSlider.SetValue` (`/Game/W_Wavetable.HighPassResKnob` _wavetable_widget) (`.HighPassFilterResonance_11_CE21AE434B54F864A7F0CBA8DCAD9E6B` (break `/Game/S_SynthSettings` _returnvalue)))
      (`Slider.SetValue` (`/Game/W_Wavetable.WaveformSlider2` _wavetable_widget) (`.Waveform2_14_2074D08C489116B87073F8A0AFB3888C` (break `/Game/S_SynthSettings` _returnvalue)))
      (`Slider.SetValue` (`/Game/W_Wavetable.AttackSlider` _wavetable_widget) (`.Attack_17_154432A54FD611843101F1B3E4759E09` (break `/Game/S_SynthSettings` _returnvalue)))
      (`Slider.SetValue` (`/Game/W_Wavetable.DecaySlider` _wavetable_widget) (`.Decay_19_7283B608499534598B1D568C6B3E68A5` (break `/Game/S_SynthSettings` _returnvalue)))
      (`Slider.SetValue` (`/Game/W_Wavetable.SustainSlider` _wavetable_widget) (`.Sustain_21_B0D73DA146EEA2A7D11E3D9A566867A3` (break `/Game/S_SynthSettings` _returnvalue)))
      (`Slider.SetValue` (`/Game/W_Wavetable.ReleaseSlider` _wavetable_widget) (`.Release_23_23CC5DFE4A601BD003110AA2AE5665CF` (break `/Game/S_SynthSettings` _returnvalue)))
      (setmembers `/Game/S_SynthSettings` :`StructRef` (`self.S Synth Settings`) :`Waveform` (break `/Game/S_SynthSettings` _returnvalue))
      (setmembers `/Game/S_SynthSettings` :`StructRef` (`self.S Synth Settings`) :`Low Pass Filter Cut Off` (* (* (`.LowPassFilterCutOff_4_6D70E24441703CD421BCE9AD6D1FC51C` (break `/Game/S_SynthSettings` _returnvalue)) 10000.0) 2.0))
      (setmembers `/Game/S_SynthSettings` :`StructRef` (`self.S Synth Settings`) :`Low Pass Filter Resonance` (`.LowPassFilterResonance_6_EA6623A744C3E250F1A0209D804692E1` (break `/Game/S_SynthSettings` _returnvalue)))
      (setmembers `/Game/S_SynthSettings` :`StructRef` (`self.S Synth Settings`) :`High Pass Filter Cut Off` (* (* (`.HighPassFilterCutOff_9_4D30AA4845A6E9CCB262F3A5AFD4EBD4` (break `/Game/S_SynthSettings` _returnvalue)) 10000.0) 2.0))
      (setmembers `/Game/S_SynthSettings` :`StructRef` (`self.S Synth Settings`) :`High Pass Filter Resonance` (`.HighPassFilterResonance_11_CE21AE434B54F864A7F0CBA8DCAD9E6B` (break `/Game/S_SynthSettings` _returnvalue)))
      (setmembers `/Game/S_SynthSettings` :`StructRef` (`self.S Synth Settings`) :`Waveform 2` (`.Waveform2_14_2074D08C489116B87073F8A0AFB3888C` (break `/Game/S_SynthSettings` _returnvalue)))
      (setmembers `/Game/S_SynthSettings` :`StructRef` (`self.S Synth Settings`) :`Attack` (`.Attack_17_154432A54FD611843101F1B3E4759E09` (break `/Game/S_SynthSettings` _returnvalue)))
      (setmembers `/Game/S_SynthSettings` :`StructRef` (`self.S Synth Settings`) :`Decay` (`.Decay_19_7283B608499534598B1D568C6B3E68A5` (break `/Game/S_SynthSettings` _returnvalue)))
      (setmembers `/Game/S_SynthSettings` :`StructRef` (`self.S Synth Settings`) :`Sustain` (`.Sustain_21_B0D73DA146EEA2A7D11E3D9A566867A3` (break `/Game/S_SynthSettings` _returnvalue)))
      (setmembers `/Game/S_SynthSettings` :`StructRef` (`self.S Synth Settings`) :`Release` (`.Release_23_23CC5DFE4A601BD003110AA2AE5665CF` (break `/Game/S_SynthSettings` _returnvalue))))))

(fn `Synth Settings`
  (params (Waveform :type "Float (double-precision)") (`Low Pass Filter Cut Off` :type "Float (double-precision)") (`Low Pass Filter Resonance` :type "Float (double-precision)") (`High Pass Filter Cut Off` :type "Float (double-precision)") (`High Pass Filter Resonance` :type "Float (double-precision)") (`Waveform 2` :type "Float (double-precision)") (`Attack Time` :type "Float (double-precision)") (`Decay Time` :type "Float (double-precision)") (`Sustain Level` :type "Float (double-precision)") (`Release Time` :type "Float (double-precision)"))
  (bind _audio (`self.Audio`))
  (`AudioComponent.SetFloatParameter` _audio "Waveform Select" Waveform)
  (`AudioComponent.SetFloatParameter` _audio "Low Pass Cutoff Frequency" `Low Pass Filter Cut Off`)
  (`AudioComponent.SetFloatParameter` _audio "Low Pass Resonance" `Low Pass Filter Resonance`)
  (`AudioComponent.SetFloatParameter` _audio "High Pass Cutoff Frequency" `High Pass Filter Cut Off`)
  (`AudioComponent.SetFloatParameter` _audio "High Pass Resonance" `High Pass Filter Resonance`)
  (`AudioComponent.SetFloatParameter` _audio "Wave Select 1" `Waveform 2`)
  (`AudioComponent.SetFloatParameter` _audio "Attack Time" `Attack Time`)
  (`AudioComponent.SetFloatParameter` _audio "Decay Time" `Decay Time`)
  (`AudioComponent.SetFloatParameter` _audio "Sustain Level" `Sustain Level`)
  (`AudioComponent.SetFloatParameter` _audio "Release Time" `Release Time`))

(fn `UserConstructionScript`)